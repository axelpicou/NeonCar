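; Drift vehicle pawn that styles itself from the Game Instance's StencilValue and drives its brake lights.
; BeginPlay uses that value to color two Niagara effects and set the mesh's custom depth stencil, then starts audio.
; A dynamic chassis material, created in the construction script, receives brake light power.
; Tick's fall reset below a Z threshold is unreachable, because its distance comparison follows an assignment equalizing both values.
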(event EventTick
  (params (DeltaSeconds :type Float%20%28single-precision%29))
  (bind _vehiclemovementcomponent (Variables|Default|GetVehicleMovementComponent))
  (bind _returnvalue (Components|GetOwner _vehiclemovementcomponent))
  (bind _returnvalue_2 (Transformation|GetActorLocation _returnvalue))
  (bind _output_get (Variables|Default|SetDistanceTotal (Variables|Default|GetDistanceOnSpline)))
  (if (< _output_get (Variables|Default|GetDistanceOnSpline))
    (Variables|Default|SetDistanceOnSpline (+ _output_get (Variables|Default|GetDistanceOnSpline)))
    (if (< (.z _returnvalue_2) -1e+03)
      (Variables|Default|SetValue%20X (.x _returnvalue_2))
      (Class|NeonCarPawn|ResetVehicle))))

(event EventBeginPlay
  (bind _asbp_game_instance (Utilities|Casting|CastTobp_GameInstance (Game|GetGameInstance)))
  (Rendering|SetRenderCustomDepth (Variables|Character|GetMesh) true)
  (switch int (Variables|/Game/bp_GameInstance.bp_GameInstance_C|GetstencilValue _asbp_game_instance)
    (:0
      (Niagara|SetNiagaraVariable(LinearColor) (Variables|Default|GetNiagara) "Linear Color" (Math|Color|MakeColor 255.0 0.0 0.0)))
    (:1
      (Niagara|SetNiagaraVariable(LinearColor) (Variables|Default|GetNiagara) "Linear Color" (Math|Color|MakeColor 0.0 1.0 0.023054)))
    (:2
      (Niagara|SetNiagaraVariable(LinearColor) (Variables|Default|GetNiagara) "Linear Color" (Math|Color|MakeColor 0.536458 0.0 0.526093)))
    (:3
      (Niagara|SetNiagaraVariable(LinearColor) (Variables|Default|GetNiagara) "Linear Color" (Math|Color|MakeColor 0.0 246.116806 255.0))))
  (Rendering|SetCustomDepthStencilValue (Variables|Character|GetMesh) (Variables|/Game/bp_GameInstance.bp_GameInstance_C|GetstencilValue _asbp_game_instance))
  (Audio|Components|Audio|SetSound (Variables|Default|GetAudio1) (Variables|Default|GetSound))
  (Audio|Components|Audio|Play (Variables|Default|GetAudio1) 0.0))

(event EventBrakeLights
  (params (bBraking :type Boolean))
  (Rendering|Material|SetScalarParameterValue (Variables|Default|GetChassis%20Material) "BrakeLightPower" (Math|Float|SelectFloat 2e+02 4.0 bBraking) :!class /Script/Engine.MaterialInstanceDynamic))

(fn ConstructionScript
  (bind _returnvalue (Rendering|Material|CreateDynamicMaterialInstance (Variables|Character|GetMesh) 0 0 "None" :!class /Script/Engine.PrimitiveComponent))
  (Variables|Default|SetChassis%20Material _returnvalue))