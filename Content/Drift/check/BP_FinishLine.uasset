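; BP_FinishLine is the race finish line trigger that counts laps for drift pawns and ends the race.
; Each pawn overlap increments that pawn's CurrentLap until it is already 3.
; The next crossing notifies the pawn, shows WBP_FinishClassement filled from BP_Manage_Race's RaceHUD and Vehicles, enables the mouse cursor and pauses the game.
; Any BP_Drift_Pawn can trigger this ending, with no check for player control.
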(event OnComponentBeginOverlap(FinishTrigger)
  (params (OverlappedComponent :type Primitive%20Component%20Object%20Reference) (OtherActor :type Actor%20Object%20Reference) (OtherComp :type Primitive%20Component%20Object%20Reference) (OtherBodyIndex :type Integer) (bFromSweep :type Boolean) (SweepResult :type Hit%20Result%20Structure%20%28by%20ref%29))
  (bind _race (Variables|Default|GetRace))
  (bind _asbp_drift_pawn (Utilities|Casting|CastToBP_Drift_Pawn OtherActor))
  (bind _output_get (Variables|Default|SetAs%20BP%20Drift%20Pawn_0 _asbp_drift_pawn))
  (if (== (Variables|/Script/NeonCar.NeonCarPawn|GetCurrentLap _output_get) 3)
    (Class|NeonCarPawn|OnCrossFinishLine _output_get)
    (bind _returnvalue (UserInterface|CreateWidget "/Game/Drift/Widget/WBP_FinishClassement.WBP_FinishClassement_C" (Game|GetPlayerController 0)))
    (UserInterface|Viewport|AddtoViewport _returnvalue 0)
    (Default|ClassementF _returnvalue (Variables|/Game/Drift/Manager/BP_Manage_Race.BP_Manage_Race_C|GetRaceHUD _race) (Variables|/Script/NeonCar.RaceManager|GetVehicles _race))
    (Variables|/Script/Engine.PlayerController|SetbShowMouseCursor (Game|GetPlayerController 0) true)
    (Game|SetGamePaused true)
    (else
      (Math|Integer|IncrementInt (Variables|/Script/NeonCar.NeonCarPawn|GetCurrentLap _output_get)))))

(event EventBeginPlay
  (bind _returnvalue (Actor|GetActorOfClass "/Game/Drift/Manager/BP_Manage_Race.BP_Manage_Race_C"))
  (Variables|Default|SetRace _returnvalue))

(fn ConstructionScript)