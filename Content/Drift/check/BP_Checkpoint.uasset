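; BP_Checkpoint is a race checkpoint actor in the drift game that detects the player's BP_Drift_Pawn on overlap.
; It finds BP_Manage_Race on BeginPlay and passes the overlapping vehicle and its own checkpoint index to the manager's ValideChecpoint.
; When that call returns true, it briefly shows the WBP_MissCheckpoint widget on the first player's screen, then removes it.
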(event Custom|ValidateCheckpoint
  (params (NewParam :type Neon%20Car%20Pawn%20Object%20Reference) (CheckpointIndex :type Integer))
  (bind _returnvalue (Class|RaceManager|ValideChecpoint (Variables|Default|GetRaceManager) NewParam CheckpointIndex))
  (if true
    (if _returnvalue
      (bind _returnvalue_2 (UserInterface|CreateWidget "/Game/Drift/Widget/WBP_MissCheckpoint.WBP_MissCheckpoint_C" (Game|GetPlayerController 0)))
      (UserInterface|Viewport|AddtoViewport _returnvalue_2 0)
      (Utilities|FlowControl|Delay 1.5)
      (Widget|RemovefromParent _returnvalue_2))))

(event EventBeginPlay
  (bind _returnvalue (Actor|GetActorOfClass "/Game/Drift/Manager/BP_Manage_Race.BP_Manage_Race_C"))
  (Variables|Default|SetRaceManager _returnvalue))

(event Collision|EventActorBeginOverlap
  (params (OtherActor :type Actor%20Object%20Reference))
  (bind _asbp_drift_pawn (Utilities|Casting|CastToBP_Drift_Pawn OtherActor))
  (bind _output_get (Variables|Default|SetAs%20BP%20Drift%20Pawn _asbp_drift_pawn))
  (CallFunction|ValidateCheckpoint _output_get (Variables|Default|GetChecpointIndex)))

(fn ConstructionScript)