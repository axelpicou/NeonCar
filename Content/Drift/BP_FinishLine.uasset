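; BP_FinishLine is a finish-line actor for the drift race that reacts when a drift pawn crosses it.
; On BeginPlay it finds the BP_Manage_Race actor and stores it.
; When a BP_Drift_Pawn overlaps it, it calls the pawn's OnCrossFinishLine, then creates a WBP_FinishClassement widget for player 0.
; The widget is added to the viewport and receives the manager's RaceHUD through ClassementF.
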(event EventBeginPlay
  (bind _returnvalue (Actor|GetActorOfClass "/Game/Drift/Manager/BP_Manage_Race.BP_Manage_Race_C"))
  (Variables|Default|SetRace _returnvalue))

(event Collision|EventActorBeginOverlap
  (params (OtherActor :type Actor%20Object%20Reference))
  (bind _asbp_drift_pawn (Utilities|Casting|CastToBP_Drift_Pawn OtherActor))
  (bind _output_get (Variables|Default|SetAs%20BP%20Drift%20Pawn _asbp_drift_pawn))
  (Class|NeonCarPawn|OnCrossFinishLine _asbp_drift_pawn)
  (bind _returnvalue (UserInterface|CreateWidget "/Game/Drift/Widget/WBP_FinishClassement.WBP_FinishClassement_C" (Game|GetPlayerController 0)))
  (UserInterface|Viewport|AddtoViewport _returnvalue 0)
  (Default|ClassementF _returnvalue (Variables|/Game/Drift/Manager/BP_Manage_Race.BP_Manage_Race_C|GetRaceHUD (Variables|Default|GetRace))))

(fn ConstructionScript)